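; BP_SurvivalGuy is an NPC that holds a voiced dialogue with the player inside its overlap sphere.
; Entering the sphere registers the NPC on the player and shows the dialogue widget; leaving ends the dialogue.
; NextLine steps through DT_SurvivalGuysDia from IndexStart, playing audio and tilting and justifying text by speaker.
; A blank or final row ends dialogue, resetting the index and clearing the player's QuestGiver, not SurvivalGuy.
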(event `self.ReceiveBeginPlay`
  (bind _returnvalue (`|CreateWidget` "/Game/Myself/NPCs/Widgets/W_SurvivalGuyDia.W_SurvivalGuyDia_C"))
  (set `self.SurvivalGuyWidget` _returnvalue)
  (set `self.LineIndex` (`self.IndexStart`)) ; Tell NPC to start at specific row
)

(event `self.Sphere.OnComponentBeginOverlap`
  (params (OverlappedComponent :type "PrimitiveComponent Object Reference") (OtherActor :type "Actor Object Reference") (OtherComp :type "PrimitiveComponent Object Reference") (OtherBodyIndex :type Integer) (bFromSweep :type Boolean) (SweepResult :type "HitResult Structure (by ref)"))
  (bind _assandbox_character_cmc1 (cast `/Game/Myself/CMC/SandboxCharacter_CMC1` OtherActor))
  (bind _output_get (set `self.Player` _assandbox_character_cmc1))
  (set `/Game/Myself/CMC/SandboxCharacter_CMC1.SurvivalGuy` self _output_get)
  (`KismetSystemLibrary.PrintText` "Hello")
  (`UserWidget.AddToViewport` (`self.SurvivalGuyWidget`) 0))

(event `Next Line`
  (bind _lineindex (`self.LineIndex`))
  (bind _audiocomponent (`self.AudioComponent`))
  (bind _textblock_0 (`/Game/Myself/NPCs/Widgets/W_SurvivalGuyDia.TextBlock_0` (`self.SurvivalGuyWidget`)))
  (bind _outrownames (`DataTableFunctionLibrary.GetDataTableRowNames` "/Game/Myself/NPCs/Blueprints/DT_SurvivalGuysDia.DT_SurvivalGuysDia"))
  (if (> _lineindex (`KismetArrayLibrary.Array_LastIndex` _outrownames))
    (`self.End Dialogue`)
    (else
      (bind _returnvalue (`|GetDataTableRow` "/Game/Myself/NPCs/Blueprints/DT_SurvivalGuysDia.DT_SurvivalGuysDia" (`|GetArrayItem` _outrownames _lineindex))
        (:`then`
          (if (`KismetTextLibrary.EqualEqual_TextText` (break `/Game/Myself/NPCs/Blueprints/S_QuestGiverDialogue` _returnvalue) "")
            (`self.End Dialogue`)
            (else
              (`TextBlock.SetText` (`/Game/Myself/NPCs/Widgets/W_SurvivalGuyDia.TextBlock_0` (`self.SurvivalGuyWidget`)) (break `/Game/Myself/NPCs/Blueprints/S_QuestGiverDialogue` _returnvalue))
              (`/Engine/EditorBlueprintResources/StandardMacros.IncrementInt` (`self.LineIndex`)
                (:`  `
                  ; Play audio, cancel previous lines if needed.
                  (`AudioComponent.SetSound` _audiocomponent (`.VoicedDialogue_5_75AD13C944973E256D7626BDFD3AAA2B` (break `/Game/Myself/NPCs/Blueprints/S_QuestGiverDialogue` _returnvalue)))
                  (`AudioComponent.Play` _audiocomponent 0.0)
                  (switch `/Game/Myself/NPCs/Blueprints/E_Speaker` (`.SpeakerStructure_9_DEA26BD849008923E0ADB9B769E9B035` (break `/Game/Myself/NPCs/Blueprints/S_QuestGiverDialogue` _returnvalue))
                    (:`NewEnumerator1`
                      (`Widget.SetRenderTransformAngle` _textblock_0 (`KismetMathLibrary.RandomFloatInRange` 2.0 3.5))
                      (set `TextLayoutWidget.Justification` "Right" _textblock_0))
                    (:`NewEnumerator3`
                      (`Widget.SetRenderTransformAngle` _textblock_0 (`KismetMathLibrary.RandomFloatInRange` -3.5 -2.0))
                      (set `TextLayoutWidget.Justification` "Left" _textblock_0))))))))))))

(event `End Dialogue`
  (`Widget.RemoveFromParent` (`self.SurvivalGuyWidget`))
  (set `self.LineIndex` (`self.IndexStart`)) ; Reset the lines
  (set `/Game/Myself/CMC/SandboxCharacter_CMC1.Quest Giver` null (`self.Player`)) ; tell the player to \nforget about us\n\nset the variable on the PC to null
  (set `self.Player` null) ; forget about the player
)

(event `self.Sphere.OnComponentEndOverlap`
  (params (OverlappedComponent :type "PrimitiveComponent Object Reference") (OtherActor :type "Actor Object Reference") (OtherComp :type "PrimitiveComponent Object Reference") (OtherBodyIndex :type Integer))
  (cast `/Game/Myself/CMC/SandboxCharacter_CMC1` OtherActor)
  (`self.End Dialogue`))

(fn `UserConstructionScript`)