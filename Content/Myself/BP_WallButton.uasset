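; BP_WallButton is a wall button actor that makes the player's right hand reach toward it on contact.
; When a SandboxCharacter_CMC1 begins overlapping its Collision component, it gets and stores the character's SandboxCharacter_CMC_ABP1 animation instance.
; It then sets that ABP's right-hand IK alpha to full and the IK target to the Button component's world location.
; No end-overlap handler resets the IK, and no press action is implemented.
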(event `self.Collision.OnComponentBeginOverlap`
  (params (OverlappedComponent :type "PrimitiveComponent Object Reference") (OtherActor :type "Actor Object Reference") (OtherComp :type "PrimitiveComponent Object Reference") (OtherBodyIndex :type Integer) (bFromSweep :type Boolean) (SweepResult :type "HitResult Structure (by ref)"))
  (bind _assandbox_character_cmc1 (cast `/Game/Myself/CMC/SandboxCharacter_CMC1` OtherActor))
  (bind _assandbox_character_cmc_abp1 (cast `/Game/Myself/CMC/SandboxCharacter_CMC_ABP1` (`SkeletalMeshComponent.GetAnimInstance` (`Character.Mesh` _assandbox_character_cmc1))))
  (set `self.ABP` _assandbox_character_cmc_abp1) ; Save this ABP as a variable
  (set `/Game/Myself/CMC/SandboxCharacter_CMC_ABP1.RightHandIK_Alpha` 1.0 (`self.ABP`))
  (set `/Game/Myself/CMC/SandboxCharacter_CMC_ABP1.RightHandIK_Target` (`SceneComponent.K2_GetComponentLocation` (`self.Button`)) (`self.ABP`)))

(fn `UserConstructionScript`)